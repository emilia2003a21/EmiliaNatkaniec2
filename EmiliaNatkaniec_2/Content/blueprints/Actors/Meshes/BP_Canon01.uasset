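; BP_Canon01 is a cannon that fires automatically and repeatedly from BeginPlay, with no targeting or trigger.
; Each cycle waits FireRate, spawns an actor at the Arrow component's location and rotation using ProjectileScale, then plays the Cannonanimation timeline.
; The timeline slides the Canon component along local Y for recoil, and its Finished pin restarts the cycle.
; SpawnProjectile (BPprojecttile04) and AnimacjaLufy (barrel animation) duplicate these steps as functions the event graph leaves uncalled.
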(event `self.ReceiveBeginPlay`
  (bind _arrow (`self.Arrow`))
  (`KismetSystemLibrary.Delay` (`self.fire rate`) :!label _label)
  (`|SpawnActorFromClass` "/Game/blueprints/Actors/BP-projecttile02.BP-projecttile02_C" (`KismetMathLibrary.MakeTransform` (`SceneComponent.K2_GetComponentLocation` _arrow) (`SceneComponent.K2_GetComponentRotation` _arrow) (`self.projectile scale`)) "Undefined" "OverrideRootScale" null null)
  (bind (_direction _canon_fired) (`Timeline|cannonanimation` :!via `PlayFromStart`)
    (:`Update`
      (`SceneComponent.K2_SetRelativeLocation` (`self.canon`) (`KismetMathLibrary.MakeVector` 0.0 _canon_fired) false false))
    (:`Finished`
      (goto _label))))

(event `self.ReceiveTick`
  (params (DeltaSeconds :type "Float (single-precision)")))

(fn `animacja lufy`
  (params (NewLocation_Y :type "Float (double-precision)"))
  (`SceneComponent.K2_SetRelativeLocation` (`self.canon`) (`KismetMathLibrary.MakeVector` 0.0 NewLocation_Y) false false))

(fn `spawnProjectile`
  (bind _arrow (`self.Arrow`))
  (`|SpawnActorFromClass` "/Game/blueprints/Actors/Meshes/BP-projecttile04.BP-projecttile04_C" (`KismetMathLibrary.MakeTransform` (`SceneComponent.K2_GetComponentLocation` _arrow) (`SceneComponent.K2_GetComponentRotation` _arrow) (`self.projectile scale`)) "Undefined" "OverrideRootScale" null null))

(fn `UserConstructionScript`)