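; BP_PlayerPawn3 is a rolling-ball player pawn that moves by applying acceleration-based torque to its sphere from the movement input axes.
; Any damage triggers a one-shot camera fade-out, then reloads the current level after a short delay.
; Two duplicate functions, AdjustCamera and Cameraadjust, set spring arm length and world pitch at a fixed yaw; neither runs within this Blueprint.
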(event `InputAxis|move left/right`
  (params (AxisValue :type "Float (single-precision)"))
  (`PrimitiveComponent.AddTorqueInRadians` (`self.Sphere`) (`KismetMathLibrary.MakeVector` 0.0 (* AxisValue (`self.multiply`))) "None" true))

(event `InputAxis|move Forward/backwards`
  (params (AxisValue :type "Float (single-precision)"))
  (`PrimitiveComponent.AddTorqueInRadians` (`self.Sphere`) (`KismetMathLibrary.MakeVector` (* AxisValue (`self.multiply`))) "None" true))

(event `self.ReceiveAnyDamage`
  (params (Damage :type "Float (single-precision)") (DamageType :type "DamageType Object Reference") (InstigatedBy :type "Controller Object Reference") (DamageCauser :type "Actor Object Reference"))
  (`/Engine/EditorBlueprintResources/StandardMacros.DoOnce` false
    (:`Completed`
      (`PlayerCameraManager.StartCameraFade` :`self` (`GameplayStatics.GetPlayerCameraManager` 0) :`ToAlpha` 1.0 :`Duration` 0.4)
      (`KismetSystemLibrary.Delay` 0.4)
      (bind _returnvalue (`GameplayStatics.GetCurrentLevelName` true))
      (`GameplayStatics.OpenLevel` (`KismetStringLibrary.Conv_StringToName` _returnvalue)))))

(fn `adjust camera`
  (params (distance :type "Float (double-precision)") (pitch :type "Float (double-precision)"))
  (bind _springarm (`self.SpringArm`))
  (set `SpringArmComponent.TargetArmLength` distance _springarm)
  (`SceneComponent.K2_SetWorldRotation` _springarm (`KismetMathLibrary.MakeRotator` 0.0 pitch 90.0) false false))

(fn `cameraadjust`
  (params (`Target Arm Length` :type "Float (double-precision)") (`Y (Pitch)` :type "Float (double-precision)"))
  (bind _springarm (`self.SpringArm`))
  (set `SpringArmComponent.TargetArmLength` `Target Arm Length` _springarm)
  (`SceneComponent.K2_SetWorldRotation` _springarm (`KismetMathLibrary.MakeRotator` 0.0 `Y (Pitch)` 90.0) false false))

(fn `NewFunction_0`)

(fn `UserConstructionScript`)