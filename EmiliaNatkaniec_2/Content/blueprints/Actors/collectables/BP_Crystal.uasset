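; BP_Crystal is a collectable crystal that flies into the player and vanishes when the player pawn overlaps its sphere.
; An IsPlayer check filters the overlap, then SetVariables caches the pawn's location and the crystal's transform and light intensity.
; A timeline lerps location toward that cached point and scale to zero, then destroys the actor.
; ChangeLights only reapplies the cached intensity, as its fade lerp is unconnected.
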(event `self.Sphere.OnComponentBeginOverlap`
  (params (OverlappedComponent :type "PrimitiveComponent Object Reference") (OtherActor :type "Actor Object Reference") (OtherComp :type "PrimitiveComponent Object Reference") (OtherBodyIndex :type Integer) (bFromSweep :type Boolean) (SweepResult :type "HitResult Structure (by ref)"))
  (`self.IsPlayer` OtherActor
    (:`IsPlayer`
      (`self.set variables`)
      (bind (_direction _crystal_location _crystal_scale _crystal_light) (`Timeline|crysrtal transform`)
        (:`Update`
          (`self.change location` _crystal_location)
          (`self.change scale` _crystal_scale)
          (`self.change lights` _crystal_light))
        (:`Finished`
          (`self.K2_DestroyActor`))))))

(fn `change lights`
  (params (Alpha :type "Float (double-precision)"))
  (`LightComponent.SetIntensity` (`self.PointLight`) (`self.crystal light`)))

(fn `change location`
  (params (Alpha :type "Float (double-precision)"))
  (`self.K2_SetActorLocation` (`KismetMathLibrary.VLerp` (`self.crystal location`) (`self.ball location`) Alpha)))

(fn `change scale`
  (params (Alpha :type "Float (double-precision)"))
  (`self.SetActorScale3D` (`KismetMathLibrary.VLerp` (`self.crystal scale`) (0.0 0.0 0.0) Alpha)))

(fn `crystal current position`
  (params (A :type "Object Object Reference"))
  (if (== A (`GameplayStatics.GetPlayerPawn` 0))
    _))

(fn `set variables`
  (set `self.ball location` (`self.K2_GetActorLocation` (`GameplayStatics.GetPlayerPawn` 0)))
  (set `self.crystal light` (`LightComponentBase.Intensity` (`self.PointLight`)))
  (set `self.crystal location` (`self.K2_GetActorLocation`))
  (set `self.crystal scale` (`self.GetActorScale3D`)))

(fn `UserConstructionScript`)

(fn `zmiana wartosci kryształu`
  (params (A :type "Object Object Reference"))
  (if (== A (`GameplayStatics.GetPlayerPawn` 0))
    _))